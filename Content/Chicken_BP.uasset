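; Player-controlled chicken pawn that moves along world X and Y with the W, A, S and D keys.
; Key presses set MoveX or MoveY from direction variables, and Tick feeds both into AddMovementInput while re-calling EnableInput.
; All keys share one stop path, run after a 0.2-second delay or on release, which resets only MoveX, so MoveY is never cleared.
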(event `self.ReceiveTick`
  (params (DeltaSeconds :type "Float (single-precision)"))
  (`self.EnableInput` null)
  (`self.AddMovementInput` (-1.0 0.0 0.0) (`self.move_x`))
  (`self.AddMovementInput` (0.0 -1.0 0.0) (`self.move_y`)))

(event `Key|A`
  (params (Key :type "Key Structure"))
  (:`Pressed`
    (set `self.move_x` (`self.left`))
    (`KismetSystemLibrary.Delay` 0.2 :!label _label)
    (set `self.move_x` (`self.stop`) :!label _label_2))
  (:`Released`
    (`self.EnableInput` null :!label _label_3)
    (goto _label_2)))

(event `Key|D`
  (params (Key :type "Key Structure"))
  (:`Pressed`
    (set `self.move_x` (`self.right`))
    (goto _label))
  (:`Released`
    (goto _label_3)))

(event `InputTouch`
  (params (Location :type "Vector Structure") (FingerIndex :type "ETouchIndex Enum")))

(event `Key|W`
  (params (Key :type "Key Structure"))
  (:`Pressed`
    (set `self.move_y` (`self.forwards`))
    (goto _label))
  (:`Released`
    (goto _label_3)))

(event `Key|S`
  (params (Key :type "Key Structure"))
  (:`Pressed`
    (set `self.move_y` (`self.backwards`))
    (goto _label))
  (:`Released`
    (goto _label_3)))

(fn `UserConstructionScript`)